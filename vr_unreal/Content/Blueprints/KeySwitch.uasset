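; KeySwitch is a VR puzzle switch that reports to the game state for a given door when activated.
; Overlapping a Grabbable_Key stores it and calls its SetKeyPlaced with the Anchor location and a switch reference; that key leaving the overlap clears the placed state.
; SwitchActivated, not called within this Blueprint, swaps the cube material for either state and, only on activation, calls PuzzleTriggered on VRGameState with its DoorIndex.
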(event `self.ReceiveActorBeginOverlap`
  (params (OtherActor :type "Actor Object Reference"))
  (bind _asgrabbable_key (cast `/Game/Blueprints/Grabbable_Key` OtherActor))
  (bind _output_get (set `self.KeyReference` _asgrabbable_key))
  (bind _output_get_2 (set `self.KeyInTrigger` true))
  (`/Game/Blueprints/Grabbable_Key.SetKeyPlaced` _output_get _output_get_2 (`SceneComponent.K2_GetComponentLocation` (`self.anchor`)) self))

(event `self.ReceiveActorEndOverlap`
  (params (OtherActor :type "Actor Object Reference"))
  (bind _keyreference (`self.KeyReference`))
  (bind _asgrabbable_key (cast `/Game/Blueprints/Grabbable_Key` OtherActor))
  (if (== _asgrabbable_key _keyreference)
    (bind _output_get (set `self.KeyInTrigger` false))
    (`/Game/Blueprints/Grabbable_Key.SetKeyPlaced` _keyreference _output_get (0.0 0.0 0.0) self)))

(fn `Switch Activated`
  (params (`Activated?` :type Boolean))
  (bind _cube (`self.Cube`))
  (if `Activated?`
    (`PrimitiveComponent.SetMaterial` _cube 0 "/Engine/VREditor/BasicMeshes/MI_Cube_02.MI_Cube_02")
    (bind _asvrgame_state (cast `/Game/Blueprints/VRGameState` (`GameplayStatics.GetGameState`)))
    (`/Game/Blueprints/VRGameState.PuzzleTriggered` _asvrgame_state (`self.DoorIndex`))
    (else
      (`PrimitiveComponent.SetMaterial` _cube 0 "/Engine/VREditor/BasicMeshes/MI_Cube_03.MI_Cube_03"))))

(fn `UserConstructionScript`)