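; TargetManager is a puzzle controller that tracks hits across a set of targets in a VR game.
; On BeginPlay it assigns itself as the manager on every entry in its Targets array.
; TargetHit increments a hit counter and, when it equals the target count, calls PuzzleTriggered on the VRGameState.
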(event `self.ReceiveBeginPlay`
  (for _array_element (`self.Targets`)
    (set `/Game/Blueprints/Target.TargetManager` self _array_element)))

(fn `TargetHit`
  (bind _result (`/Engine/EditorBlueprintResources/StandardMacros.IncrementInt` (`self.targetHits`))
    (:`  `
      (if (== _result (`KismetArrayLibrary.Array_Length` (`self.Targets`)))
        (bind _asvrgame_state (cast `/Game/Blueprints/VRGameState` (`GameplayStatics.GetGameState`)))
        (`/Game/Blueprints/VRGameState.PuzzleTriggered` _asvrgame_state)
        (else
          (return))))))

(fn `UserConstructionScript`)