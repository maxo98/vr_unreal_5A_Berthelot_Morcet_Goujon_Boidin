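; Pressure-plate trigger for a VR puzzle that activates once when a Movable_BigCube hits it.
; On the hit it tells the cube it is placed, swaps the plate material, and plays a timeline that moves the button mesh down.
; When the press animation finishes, it notifies VRGameState that a puzzle step has triggered.
; The DoOnce sits before the cast, so the first hit of any actor consumes the trigger.
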(event `self.ReceiveHit`
  (params (MyComp :type "PrimitiveComponent Object Reference") (Other :type "Actor Object Reference") (OtherComp :type "PrimitiveComponent Object Reference") (bSelfMoved :type Boolean) (HitLocation :type "Vector Structure") (HitNormal :type "Vector Structure") (NormalImpulse :type "Vector Structure") (Hit :type "HitResult Structure (by ref)"))
  (`/Engine/EditorBlueprintResources/StandardMacros.DoOnce` false
    (:`Completed`
      (bind _asmovable_big_cube (cast `/Game/Blueprints/Movable_BigCube` Other))
      (`/Game/Blueprints/Movable_BigCube.CubePlaced` _asmovable_big_cube)
      (`PrimitiveComponent.SetMaterial` (`self.Cube`) 0 "/Game/Materials/MI_Cube_04.MI_Cube_04")
      (bind (_direction _press) (`Timeline|ButtonPress`)
        (:`Update`
          (`SceneComponent.K2_SetRelativeLocation` (`self.Cube1`) _press false false))
        (:`Finished`
          (bind _asvrgame_state (cast `/Game/Blueprints/VRGameState` (`GameplayStatics.GetGameState`)))
          (`/Game/Blueprints/VRGameState.PuzzleTriggered` _asvrgame_state))))))

(fn `UserConstructionScript`)