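; VR player pawn that handles teleport movement, snap turning, object grabbing, a toggleable menu and animated hand poses through Enhanced Input.
; Teleport traces a projectile arc from the right controller into a Niagara trail, validating the landing on the navmesh.
; Snap turn and teleport compensate for the camera's offset within the pawn.
; Grabbing sphere-traces physics bodies for the nearest GrabComponent, while hand inputs drive pose alphas on the hand AnimBPs.
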(event `self.ReceiveBeginPlay`
  (bind _returnvalue (pcsubsystem `EnhancedInputLocalPlayerSubsystem` (`GameplayStatics.GetPlayerController` 0)))
  (if (`HeadMountedDisplayFunctionLibrary.IsHeadMountedDisplayEnabled`)
    (`HeadMountedDisplayFunctionLibrary.SetTrackingOrigin` "Stage")
    (`KismetSystemLibrary.ExecuteConsoleCommand` "vr.PixelDensity 1.0" null)
    (`EnhancedInputSubsystemInterface.AddMappingContext` _returnvalue "/Game/Input/IMC_Default.IMC_Default" 0 (struct))
    (`EnhancedInputSubsystemInterface.AddMappingContext` _returnvalue "/Game/Input/IMC_Hands.IMC_Hands" 0 (struct))))

(event `EnhancedInput|/Game/Input/Actions/IA_Turn`
  (params (ActionValue :type "Float (double-precision)") (ElapsedSeconds :type "Float (double-precision)") (TriggeredSeconds :type "Float (double-precision)") (InputAction :type "InputAction Object Reference" :default "/Game/Input/Actions/IA_Turn.IA_Turn"))
  (:`Started`
    (`self.SnapTurn` (> ActionValue 0.0))))

(event `EnhancedInput|/Game/Input/Actions/IA_Move`
  (params (ActionValue :type "Float (double-precision)") (ElapsedSeconds :type "Float (double-precision)") (TriggeredSeconds :type "Float (double-precision)") (InputAction :type "InputAction Object Reference" :default "/Game/Input/Actions/IA_Move.IA_Move"))
  (bind _motioncontrollerrightaim (`self.MotionControllerRightAim`))
  (:`Triggered`
    (`self.TeleportTrace` (`SceneComponent.K2_GetComponentLocation` _motioncontrollerrightaim) (`SceneComponent.GetForwardVector` _motioncontrollerrightaim)))
  (:`Started`
    (`self.StartTeleportTrace`))
  (:`Completed`
    (`self.EndTeleportTrace`)
    (`self.TryTeleport`)))

(event `EnhancedInput|/Game/Input/Actions/IA_Grab_Left`
  (params (ActionValue :type "Float (double-precision)") (ElapsedSeconds :type "Float (double-precision)") (TriggeredSeconds :type "Float (double-precision)") (InputAction :type "InputAction Object Reference" :default "/Game/Input/Actions/IA_Grab_Left.IA_Grab_Left"))
  (:`Started`
    (bind _nearestcomponent (`self.Get Grab Component Near Motion Controller` (`self.MotionControllerLeft`)))
    (`/Engine/EditorBlueprintResources/StandardMacros.IsValid` _nearestcomponent
      (:`Is Valid`
        (bind _isheld (`/Game/Blueprints/GrabComponent.TryGrab` _nearestcomponent (`self.MotionControllerLeft`)))
        (if _isheld
          (set `self.HeldComponentLeft` _nearestcomponent)
          (if (== (`self.HeldComponentLeft`) (`self.HeldComponentRight`))
            (set `self.HeldComponentRight` null))))))
  (:`Completed`
    (bind _heldcomponentleft (`self.HeldComponentLeft`)
      (:`then`
        (bind _breleased (`/Game/Blueprints/GrabComponent.TryRelease` _heldcomponentleft))
        (if _breleased
          (set `self.HeldComponentLeft` null)))
      (:`else`))))

(event `EnhancedInput|/Game/Input/Actions/IA_Grab_Right`
  (params (ActionValue :type "Float (double-precision)") (ElapsedSeconds :type "Float (double-precision)") (TriggeredSeconds :type "Float (double-precision)") (InputAction :type "InputAction Object Reference" :default "/Game/Input/Actions/IA_Grab_Right.IA_Grab_Right"))
  (:`Started`
    (bind _nearestcomponent (`self.Get Grab Component Near Motion Controller` (`self.MotionControllerRight`)))
    (`/Engine/EditorBlueprintResources/StandardMacros.IsValid` _nearestcomponent
      (:`Is Valid`
        (bind _isheld (`/Game/Blueprints/GrabComponent.TryGrab` _nearestcomponent (`self.MotionControllerRight`)))
        (if _isheld
          (set `self.HeldComponentRight` _nearestcomponent)
          (if (== (`self.HeldComponentRight`) (`self.HeldComponentLeft`))
            (set `self.HeldComponentLeft` null))))))
  (:`Completed`
    (bind _heldcomponentright (`self.HeldComponentRight`)
      (:`then`
        (bind _breleased (`/Game/Blueprints/GrabComponent.TryRelease` _heldcomponentright))
        (if _breleased
          (set `self.HeldComponentRight` null)))
      (:`else`))))

(event `EnhancedInput|/Game/Input/Actions/IA_Menu_Toggle_Left`
  (params (ActionValue :type Boolean) (ElapsedSeconds :type "Float (double-precision)") (TriggeredSeconds :type "Float (double-precision)") (InputAction :type "InputAction Object Reference" :default "/Game/Input/Actions/IA_Menu_Toggle_Left.IA_Menu_Toggle_Left"))
  (:`Started`
    (`self.ToggleMenu` false)))

(event `EnhancedInput|/Game/Input/Actions/IA_Menu_Toggle_Right`
  (params (ActionValue :type Boolean) (ElapsedSeconds :type "Float (double-precision)") (TriggeredSeconds :type "Float (double-precision)") (InputAction :type "InputAction Object Reference" :default "/Game/Input/Actions/IA_Menu_Toggle_Right.IA_Menu_Toggle_Right"))
  (:`Started`
    (`self.ToggleMenu` true)))

(event `EnhancedInput|/Game/Input/Actions/Hands/IA_Hand_Grasp_Left`
  (params (ActionValue :type "Float (double-precision)") (ElapsedSeconds :type "Float (double-precision)") (TriggeredSeconds :type "Float (double-precision)") (InputAction :type "InputAction Object Reference" :default "/Game/Input/Actions/Hands/IA_Hand_Grasp_Left.IA_Hand_Grasp_Left"))
  (bind _returnvalue (`SkeletalMeshComponent.GetAnimInstance` (`self.HandLeft`)))
  (:`Triggered`
    (bind _asabp_mannequins_xr (cast `/Game/Characters/MannequinsXR/Meshes/ABP_MannequinsXR` _returnvalue))
    (set `/Game/Characters/MannequinsXR/Meshes/ABP_MannequinsXR.PoseAlphaGrasp` ActionValue _asabp_mannequins_xr))
  (:`Canceled`
    (bind _asabp_mannequins_xr_2 (cast `/Game/Characters/MannequinsXR/Meshes/ABP_MannequinsXR` _returnvalue :!label _label))
    (set `/Game/Characters/MannequinsXR/Meshes/ABP_MannequinsXR.PoseAlphaGrasp` 0.0 _asabp_mannequins_xr_2))
  (:`Completed`
    (goto _label)))

(event `EnhancedInput|/Game/Input/Actions/Hands/IA_Hand_Grasp_Right`
  (params (ActionValue :type "Float (double-precision)") (ElapsedSeconds :type "Float (double-precision)") (TriggeredSeconds :type "Float (double-precision)") (InputAction :type "InputAction Object Reference" :default "/Game/Input/Actions/Hands/IA_Hand_Grasp_Right.IA_Hand_Grasp_Right"))
  (bind _returnvalue (`SkeletalMeshComponent.GetAnimInstance` (`self.HandRight`)))
  (:`Triggered`
    (bind _asabp_mannequins_xr (cast `/Game/Characters/MannequinsXR/Meshes/ABP_MannequinsXR` _returnvalue))
    (set `/Game/Characters/MannequinsXR/Meshes/ABP_MannequinsXR.PoseAlphaGrasp` ActionValue _asabp_mannequins_xr))
  (:`Canceled`
    (bind _asabp_mannequins_xr_2 (cast `/Game/Characters/MannequinsXR/Meshes/ABP_MannequinsXR` _returnvalue :!label _label_2))
    (set `/Game/Characters/MannequinsXR/Meshes/ABP_MannequinsXR.PoseAlphaGrasp` 0.0 _asabp_mannequins_xr_2))
  (:`Completed`
    (goto _label_2)))

(event `EnhancedInput|/Game/Input/Actions/Hands/IA_Hand_IndexCurl_Left`
  (params (ActionValue :type "Float (double-precision)") (ElapsedSeconds :type "Float (double-precision)") (TriggeredSeconds :type "Float (double-precision)") (InputAction :type "InputAction Object Reference" :default "/Game/Input/Actions/Hands/IA_Hand_IndexCurl_Left.IA_Hand_IndexCurl_Left"))
  (bind _returnvalue (`SkeletalMeshComponent.GetAnimInstance` (`self.HandLeft`)))
  (:`Triggered`
    (bind _asabp_mannequins_xr (cast `/Game/Characters/MannequinsXR/Meshes/ABP_MannequinsXR` _returnvalue))
    (set `/Game/Characters/MannequinsXR/Meshes/ABP_MannequinsXR.PoseAlphaIndexCurl` ActionValue _asabp_mannequins_xr))
  (:`Canceled`
    (bind _asabp_mannequins_xr_2 (cast `/Game/Characters/MannequinsXR/Meshes/ABP_MannequinsXR` _returnvalue :!label _label_3))
    (set `/Game/Characters/MannequinsXR/Meshes/ABP_MannequinsXR.PoseAlphaIndexCurl` 0.0 _asabp_mannequins_xr_2))
  (:`Completed`
    (goto _label_3)))

(event `EnhancedInput|/Game/Input/Actions/Hands/IA_Hand_IndexCurl_Right`
  (params (ActionValue :type "Float (double-precision)") (ElapsedSeconds :type "Float (double-precision)") (TriggeredSeconds :type "Float (double-precision)") (InputAction :type "InputAction Object Reference" :default "/Game/Input/Actions/Hands/IA_Hand_IndexCurl_Right.IA_Hand_IndexCurl_Right"))
  (bind _returnvalue (`SkeletalMeshComponent.GetAnimInstance` (`self.HandRight`)))
  (:`Triggered`
    (bind _asabp_mannequins_xr (cast `/Game/Characters/MannequinsXR/Meshes/ABP_MannequinsXR` _returnvalue))
    (set `/Game/Characters/MannequinsXR/Meshes/ABP_MannequinsXR.PoseAlphaIndexCurl` ActionValue _asabp_mannequins_xr))
  (:`Canceled`
    (bind _asabp_mannequins_xr_2 (cast `/Game/Characters/MannequinsXR/Meshes/ABP_MannequinsXR` _returnvalue :!label _label_4))
    (set `/Game/Characters/MannequinsXR/Meshes/ABP_MannequinsXR.PoseAlphaIndexCurl` 0.0 _asabp_mannequins_xr_2))
  (:`Completed`
    (goto _label_4)))

(event `EnhancedInput|/Game/Input/Actions/Hands/IA_Hand_Point_Left`
  (params (ActionValue :type "Float (double-precision)") (ElapsedSeconds :type "Float (double-precision)") (TriggeredSeconds :type "Float (double-precision)") (InputAction :type "InputAction Object Reference" :default "/Game/Input/Actions/Hands/IA_Hand_Point_Left.IA_Hand_Point_Left"))
  (:`Started`
    (bind _asabp_mannequins_xr (cast `/Game/Characters/MannequinsXR/Meshes/ABP_MannequinsXR` (`SkeletalMeshComponent.GetAnimInstance` (`self.HandLeft`)) :!label _label_5))
    (set `/Game/Characters/MannequinsXR/Meshes/ABP_MannequinsXR.PoseAlphaPoint` 0.0 _asabp_mannequins_xr))
  (:`Canceled`
    (goto _label_5))
  (:`Completed`
    (bind _asabp_mannequins_xr_2 (cast `/Game/Characters/MannequinsXR/Meshes/ABP_MannequinsXR` (`SkeletalMeshComponent.GetAnimInstance` (`self.HandLeft`))))
    (set `/Game/Characters/MannequinsXR/Meshes/ABP_MannequinsXR.PoseAlphaPoint` 1.0 _asabp_mannequins_xr_2)))

(event `EnhancedInput|/Game/Input/Actions/Hands/IA_Hand_Point_Right`
  (params (ActionValue :type "Float (double-precision)") (ElapsedSeconds :type "Float (double-precision)") (TriggeredSeconds :type "Float (double-precision)") (InputAction :type "InputAction Object Reference" :default "/Game/Input/Actions/Hands/IA_Hand_Point_Right.IA_Hand_Point_Right"))
  (bind _handright (`self.HandRight`))
  (:`Started`
    (bind _asabp_mannequins_xr (cast `/Game/Characters/MannequinsXR/Meshes/ABP_MannequinsXR` (`SkeletalMeshComponent.GetAnimInstance` _handright) :!label _label_6))
    (set `/Game/Characters/MannequinsXR/Meshes/ABP_MannequinsXR.PoseAlphaPoint` 0.0 _asabp_mannequins_xr))
  (:`Canceled`
    (goto _label_6))
  (:`Completed`
    (bind _asabp_mannequins_xr_2 (cast `/Game/Characters/MannequinsXR/Meshes/ABP_MannequinsXR` (`SkeletalMeshComponent.GetAnimInstance` _handright)))
    (set `/Game/Characters/MannequinsXR/Meshes/ABP_MannequinsXR.PoseAlphaPoint` 1.0 _asabp_mannequins_xr_2)))

(event `EnhancedInput|/Game/Input/Actions/Hands/IA_Hand_ThumbUp_Left`
  (params (ActionValue :type "Float (double-precision)") (ElapsedSeconds :type "Float (double-precision)") (TriggeredSeconds :type "Float (double-precision)") (InputAction :type "InputAction Object Reference" :default "/Game/Input/Actions/Hands/IA_Hand_ThumbUp_Left.IA_Hand_ThumbUp_Left"))
  (:`Started`
    (bind _asabp_mannequins_xr (cast `/Game/Characters/MannequinsXR/Meshes/ABP_MannequinsXR` (`SkeletalMeshComponent.GetAnimInstance` (`self.HandLeft`)) :!label _label_7))
    (set `/Game/Characters/MannequinsXR/Meshes/ABP_MannequinsXR.PoseAlphaThumbUp` 0.0 _asabp_mannequins_xr))
  (:`Canceled`
    (goto _label_7))
  (:`Completed`
    (bind _asabp_mannequins_xr_2 (cast `/Game/Characters/MannequinsXR/Meshes/ABP_MannequinsXR` (`SkeletalMeshComponent.GetAnimInstance` (`self.HandLeft`))))
    (set `/Game/Characters/MannequinsXR/Meshes/ABP_MannequinsXR.PoseAlphaThumbUp` 1.0 _asabp_mannequins_xr_2)))

(event `EnhancedInput|/Game/Input/Actions/Hands/IA_Hand_ThumbUp_Right`
  (params (ActionValue :type "Float (double-precision)") (ElapsedSeconds :type "Float (double-precision)") (TriggeredSeconds :type "Float (double-precision)") (InputAction :type "InputAction Object Reference" :default "/Game/Input/Actions/Hands/IA_Hand_ThumbUp_Right.IA_Hand_ThumbUp_Right"))
  (bind _handright (`self.HandRight`))
  (:`Started`
    (bind _asabp_mannequins_xr (cast `/Game/Characters/MannequinsXR/Meshes/ABP_MannequinsXR` (`SkeletalMeshComponent.GetAnimInstance` _handright) :!label _label_8))
    (set `/Game/Characters/MannequinsXR/Meshes/ABP_MannequinsXR.PoseAlphaThumbUp` 0.0 _asabp_mannequins_xr))
  (:`Canceled`
    (goto _label_8))
  (:`Completed`
    (bind _asabp_mannequins_xr_2 (cast `/Game/Characters/MannequinsXR/Meshes/ABP_MannequinsXR` (`SkeletalMeshComponent.GetAnimInstance` _handright)))
    (set `/Game/Characters/MannequinsXR/Meshes/ABP_MannequinsXR.PoseAlphaThumbUp` 1.0 _asabp_mannequins_xr_2)))

(fn `EndTeleportTrace`
  (set `self.bTeleportTraceActive` false)
  (bind _teleportvisualizerreference (`self.TeleportVisualizerReference`)
    (:`then`
      (`self.K2_DestroyActor` _teleportvisualizerreference) ; Destroy teleport Visualizer
    )
    (:`else`
      _))
  (`SceneComponent.SetVisibility` (`self.TeleportationTraceNiagaraSystem`) false false) ; Hide the teleport trace
)

(fn `Get Grab Component Near Motion Controller`
  (params (MotionController :type "MotionControllerComponent Object Reference"))
  (returns (NearestComponent :type "/Game/Blueprints/GrabComponent Object Reference"))
  (locals (LocalNearestGrabComponent :type "/Game/Blueprints/GrabComponent Object Reference") (LocalGripPosition :type "Vector Structure") (LocalGrabComponents :type "Array of /Game/Blueprints/GrabComponent Object Reference") (LocalNearestComponentDistance :type "Float (double-precision)" :default 9999999.0))
  (`|ExecutionSequence`
    (:`then_0`
      (bind _output_get (set `local.LocalGripPosition` (`SceneComponent.K2_GetComponentLocation` MotionController)))
      (bind (_outhit _returnvalue) (`KismetSystemLibrary.SphereTraceSingleForObjects` :`Start` _output_get :`End` _output_get :`Radius` (`self.GrabRadiusFromGripPosition`) :`ObjectTypes` (`|MakeArray` "ObjectTypeQuery4" :!type "EObjectTypeQuery Enum") :`TraceColor` (struct :`G` 1.0 :`B` 1.0 :`A` 1.0) :`DrawTime` 1.0))
      (if _returnvalue
        (bind _returnvalue_2 (`self.K2_GetComponentsByClass` (`.HitActor` (`GameplayStatics.BreakHitResult` _outhit)) "/Game/Blueprints/GrabComponent.GrabComponent_C"))
        (if (> (`KismetArrayLibrary.Array_Length` _returnvalue_2) 0)
          (bind _output_get_2 (set `local.LocalGrabComponents` _returnvalue_2))
          (for _array_element _output_get_2
            (bind _returnvalue_3 (`KismetMathLibrary.VSizeSquared` (- (`SceneComponent.K2_GetComponentLocation` _array_element) (`local.LocalGripPosition`))))
            (if (<= _returnvalue_3 (`local.LocalNearestComponentDistance`))
              (set `local.LocalNearestComponentDistance` _returnvalue_3)
              (set `local.LocalNearestGrabComponent` _array_element))))))
    (:`then_1`
      (return (`local.LocalNearestGrabComponent`)) ; Return nearest component
    )))

(fn `IsValidTeleportLocation`
  (params (Hit :type "HitResult Structure (by ref)"))
  (returns (ProjectedLocation :type "Vector Structure") (ReturnValue :type Boolean))
  (bind (_projectedlocation _returnvalue) (`NavigationSystemV1.K2_ProjectPointToNavigation` (`NavigationSystemV1.GetNavigationSystem`) (`.Location` (`GameplayStatics.BreakHitResult` Hit)) null null (`self.TeleportProjectPointNavigationQueryExtent`)))
  (return _projectedlocation _returnvalue))

(fn `SnapTurn`
  (params (bRightTurn :type Boolean))
  (locals (LocalCameraLocation :type "Vector Structure") (LocalCameraRelativeTransform :type "Transform Structure") (LocalYawDelta :type "Float (double-precision)") (LocalNewTransform :type "Transform Structure"))
  (bind _camera (`self.Camera`))
  (bind _snapturndegrees (`self.SnapTurnDegrees`))
  (bind _returnvalue_location (`KismetMathLibrary.BreakTransform` (`KismetMathLibrary.ComposeTransforms` (`local.LocalCameraRelativeTransform`) (`local.LocalNewTransform`))))
  (set `local.LocalYawDelta` (`KismetMathLibrary.SelectFloat` (`KismetMathLibrary.Abs` _snapturndegrees) _snapturndegrees (`local.bRightTurn`)))
  (set `local.LocalCameraLocation` (`SceneComponent.K2_GetComponentLocation` _camera))
  (set `local.LocalCameraRelativeTransform` (`SceneComponent.GetRelativeTransform` _camera))
  (set `local.LocalNewTransform` (`KismetMathLibrary.MakeTransform` (`self.K2_GetActorLocation`) (`KismetMathLibrary.ComposeRotators` (`self.K2_GetActorRotation`) (`KismetMathLibrary.MakeRotator` 0.0 0.0 (`local.LocalYawDelta`)))))
  (`self.K2_AddActorWorldRotation` (`KismetMathLibrary.MakeRotator` 0.0 0.0 (`local.LocalYawDelta`)) false true)
  (`self.K2_SetActorLocation` (+ (- (`local.LocalCameraLocation`) _returnvalue_location) (`self.K2_GetActorLocation`)) false true))

(fn `StartTeleportTrace`
  (set `self.bTeleportTraceActive` true)
  (`SceneComponent.SetVisibility` (`self.TeleportationTraceNiagaraSystem`) true false)
  (bind _returnvalue (`|SpawnActorFromClass` "/Game/Blueprints/VRTeleportVisualizer.VRTeleportVisualizer_C" (`KismetMathLibrary.MakeTransform` (0.0 0.0 0.0)) "Undefined" "OverrideRootScale" self null))
  (set `self.TeleportVisualizerReference` _returnvalue))

(fn `TeleportTrace`
  (params (StartPos :type "Vector Structure") (ForwardVector :type "Vector Structure"))
  (locals (LocalTeleportLaunchSpeed :type "Float (double-precision)" :default 650.0) (LocalNavMeshCellHeight :type "Float (double-precision)" :default 8.0) (LocalTeleportProjectileRadius :type "Float (double-precision)" :default 3.6))
  (`|ExecutionSequence`
    (:`then_0`
      (bind (_outhit _outpathpositions) (`GameplayStatics.Blueprint_PredictProjectilePath_ByObjectType` StartPos (* (`KismetMathLibrary.Conv_DoubleToVector` (`local.LocalTeleportLaunchSpeed`)) ForwardVector) true (`local.LocalTeleportProjectileRadius`) (`|MakeArray` "ObjectTypeQuery1" :!type "EObjectTypeQuery Enum") false (`|MakeArray` null :!type "Actor Object Reference")))
      (bind _output_get (set `self.TeleportTracePathPositions` _outpathpositions))
      (`KismetArrayLibrary.Array_Insert` _output_get (`local.StartPos`))
      (bind (_projectedlocation _returnvalue) (`self.IsValidTeleportLocation` _outhit))
      (set `self.ProjectedTeleportLocation` (`KismetMathLibrary.MakeVector` (.x _projectedlocation) (.y _projectedlocation) (- (.z _projectedlocation) (`local.LocalNavMeshCellHeight`))))
      (if (!= (`self.bValidTeleportLocation`) _returnvalue)
        (set `self.bValidTeleportLocation` _returnvalue)
        (`SceneComponent.SetVisibility` (`Actor.RootComponent` (`self.TeleportVisualizerReference`)) (`self.bValidTeleportLocation`) true)))
    (:`then_1`
      (`self.K2_SetActorLocation` (`self.TeleportVisualizerReference`) (`self.ProjectedTeleportLocation`) false false)
      (`NiagaraDataInterfaceArrayFunctionLibrary.SetNiagaraArrayVector` (`self.TeleportationTraceNiagaraSystem`) "User.PointArray" (`self.TeleportTracePathPositions`))
      (return))))

(fn `ToggleMenu`
  (params (bActiveMenuHandRight :type Boolean))
  (`self.MenuReference`
    (:`then`
      (`/Game/Blueprints/Menu.CloseMenu` (`self.MenuReference`)))
    (:`else`
      (bind _returnvalue (`|SpawnActorFromClass` "/Game/Blueprints/Menu.Menu_C" (`KismetMathLibrary.MakeTransform` (0.0 0.0 0.0)) "Undefined" "OverrideRootScale" null bActiveMenuHandRight self))
      (set `self.MenuReference` _returnvalue))))

(fn `TryTeleport`
  (bind (_returnvalue_roll _returnvalue_pitch _returnvalue_yaw) (`KismetMathLibrary.BreakRotator` (`self.K2_GetActorRotation`)))
  (if (`self.bValidTeleportLocation`)
    (set `self.bValidTeleportLocation` false)
    (`self.K2_TeleportTo` (- (`self.ProjectedTeleportLocation`) (`KismetMathLibrary.GreaterGreater_VectorRotator` (`KismetMathLibrary.MakeVector` (.x (`SceneComponent.RelativeLocation` (`self.Camera`))) (.y (`SceneComponent.RelativeLocation` (`self.Camera`)))) (`KismetMathLibrary.MakeRotator` 0.0 0.0 _returnvalue_yaw))) (`KismetMathLibrary.MakeRotator` 0.0 0.0 _returnvalue_yaw))))

(fn `UserConstructionScript`)