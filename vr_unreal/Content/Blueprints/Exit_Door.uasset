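; Exit door that unlocks and slides open once enough triggers have been validated.
; BeginPlay gathers three point lights and their support meshes into parallel arrays.
; Each OnTriggerValidated call turns the next light green, swaps its support material and increments a counter.
; When the counter matches the light count, OpenDoor changes the door's material and plays a timeline that moves it.
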(event `self.ReceiveBeginPlay`
  (bind _lights (`self.Lights`))
  (bind _lightsupports (`self.LightSupports`))
  (`KismetArrayLibrary.Array_AddUnique` _lights (`self.PointLight`))
  (`KismetArrayLibrary.Array_AddUnique` _lights (`self.PointLight1`))
  (`KismetArrayLibrary.Array_AddUnique` _lights (`self.PointLight2`))
  (`KismetArrayLibrary.Array_AddUnique` _lightsupports (`self.Light1`))
  (`KismetArrayLibrary.Array_AddUnique` _lightsupports (`self.Light2`))
  (`KismetArrayLibrary.Array_AddUnique` _lightsupports (`self.Light3`)))

(event `OpenDoor`
  (`PrimitiveComponent.SetMaterial` (`self.Door`) 0 "/Engine/VREditor/BasicMeshes/MI_Cube_04.MI_Cube_04")
  (bind (_direction _movedoor) (`Timeline|SlideDoor`)
    (:`Update`
      (`SceneComponent.K2_SetRelativeLocation` (`self.Door`) _movedoor false false))))

(fn `OnTriggerValidated`
  (`LightComponent.SetLightColor` (`|GetArrayItem` (`self.Lights`) (`self.CountLightActivated`)) (struct :`G` 1.0 :`A` 1.0) true)
  (`PrimitiveComponent.SetMaterial` (`|GetArrayItem` (`self.LightSupports`) (`self.CountLightActivated`)) 0 "/Engine/VREditor/BasicMeshes/MI_Ball_03.MI_Ball_03")
  (bind _result (`/Engine/EditorBlueprintResources/StandardMacros.IncrementInt` (`self.CountLightActivated`))
    (:`  `
      (if (== _result (`KismetArrayLibrary.Array_Length` (`self.Lights`)))
        (`self.OpenDoor`)))))

(fn `UserConstructionScript`)