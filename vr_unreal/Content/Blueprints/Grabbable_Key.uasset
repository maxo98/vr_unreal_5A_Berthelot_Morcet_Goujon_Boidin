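; Grabbable key that snaps onto a switch when released in a placed state, and otherwise falls with physics.
; SetKeyPlaced stores the placed flag, snap position and Switch reference used by the GrabComponent drop and grab events.
; A placed drop disables physics, teleports and zeroes rotation, swaps the material and notifies the Switch of its color change.
; Grabbing a placed key swaps the material again and turns the Switch color off.
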(event `self.GrabComponent.OnDropped`
  (bind _staticmesh (`self.StaticMesh`))
  (bind _staticmesh_2 (`self.StaticMesh`))
  (if (`self.IsPlaced`)
    (`PrimitiveComponent.SetEnableGravity` _staticmesh_2 false)
    (`PrimitiveComponent.SetSimulatePhysics` _staticmesh_2 false)
    (`PrimitiveComponent.SetMaterial` _staticmesh_2 0 "/Engine/VREditor/BasicMeshes/MI_Cube_02.MI_Cube_02")
    (`self.K2_SetActorLocation` (`self.KeyPositionOnSwitch`) false true)
    (`self.K2_SetActorRotation` (struct))
    (`/Game/Blueprints/KeySwitch.Color Switch Changed` (`self.Switch`) true)
    (else
      (`PrimitiveComponent.SetEnableGravity` _staticmesh true)
      (`PrimitiveComponent.SetSimulatePhysics` _staticmesh true))))

(event `self.GrabComponent.OnGrabbed`
  (if (`self.IsPlaced`)
    (`PrimitiveComponent.SetMaterial` (`self.StaticMesh`) 0 "/Engine/VREditor/BasicMeshes/MI_Cube_03.MI_Cube_03")
    (`/Game/Blueprints/KeySwitch.Color Switch Changed` (`self.Switch`) false)))

(fn `SetKeyPlaced`
  (params (bKeySet :type Boolean) (KeyPosition :type "Vector Structure") (switch :type "/Game/Blueprints/KeySwitch Object Reference"))
  (set `self.IsPlaced` bKeySet)
  (set `self.KeyPositionOnSwitch` KeyPosition)
  (set `self.Switch` switch))

(fn `UserConstructionScript`
  (`parent.UserConstructionScript`))