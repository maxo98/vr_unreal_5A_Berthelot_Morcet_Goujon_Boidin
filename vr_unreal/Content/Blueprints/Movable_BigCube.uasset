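; Movable big cube for VR that slides along a straight track when grabbed with a motion controller.
; The segment's endpoints come from the first two spline points at BeginPlay.
; Grabbing detaches the actor, stores an X-only hand offset and enables Tick, which snaps the mesh to the segment's closest point to the offset controller until dropping disables Tick.
; CubePlaced swaps the mesh material.
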(event `self.ReceiveBeginPlay`
  (bind _spline (`self.Spline`))
  (set `self.StartPos` (`SplineComponent.GetLocationAtSplinePoint` _spline 1 "World"))
  (set `self.EndPos` (`SplineComponent.GetLocationAtSplinePoint` _spline 0 "World")))

(event `self.ReceiveTick`
  (params (DeltaSeconds :type "Float (single-precision)"))
  (bind _grabcomponent (`self.GrabComponent`))
  (if (`/Game/Blueprints/GrabComponent.bIsHeld` _grabcomponent)
    (`SceneComponent.K2_SetWorldLocation` (`self.StaticMesh`) (`KismetMathLibrary.FindClosestPointOnSegment` (+ (`SceneComponent.K2_GetComponentLocation` (`/Game/Blueprints/GrabComponent.MotionControllerRef` _grabcomponent)) (`self.OffsetPos`)) (`self.StartPos`) (`self.EndPos`)) false false)))

(event `self.GrabComponent.OnGrabbed`
  (bind _returnvalue_x (`KismetMathLibrary.BreakVector` (`SceneComponent.K2_GetComponentLocation` (`self.StaticMesh`))))
  (bind _returnvalue_x_2 (`KismetMathLibrary.BreakVector` (`SceneComponent.K2_GetComponentLocation` (`/Game/Blueprints/GrabComponent.MotionControllerRef` (`self.GrabComponent`)))))
  (`self.K2_DetachFromActor` "KeepWorld" "KeepWorld" "KeepWorld")
  (`self.SetActorTickEnabled` true)
  (set `self.OffsetPos` (`KismetMathLibrary.MakeVector` (- _returnvalue_x _returnvalue_x_2))))

(event `self.GrabComponent.OnDropped`
  (`self.SetActorTickEnabled` false))

(fn `CubePlaced`
  (`PrimitiveComponent.SetMaterial` (`self.StaticMesh`) 0 "/Engine/VREditor/BasicMeshes/MI_Cube_04.MI_Cube_04"))

(fn `UserConstructionScript`)